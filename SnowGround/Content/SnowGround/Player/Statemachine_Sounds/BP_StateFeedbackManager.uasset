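; Feedback manager that reacts to the player character's locomotion state changes with sounds and debug prints.
; On BeginPlay it casts player 0 to BP_ThirdPersonCharacter and binds a handler to its locomotion state change dispatcher.
; The handler switches on the new state, printing each one and adding an audio component for Sprint, Jump, Fall and Landed, while Move and Idle only print.
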(event Custom|HandleLocomotionstatechange
  (params (New%20State :type E_LocomotionState%20Enum :default "NewEnumerator0"))
  (switch Utilities|FlowControl|Switch|SwitchonE_LocomotionState New%20State
    (:NewEnumerator0
      (Development|PrintString "State:Moving"))
    (:NewEnumerator3
      (Development|PrintString "State: Idle"))
    (:NewEnumerator4
      (Development|PrintString "State:Sprint")
      (AddComponent|AddAudioComponent false))
    (:NewEnumerator1
      (Development|PrintString "State:Jump")
      (AddComponent|AddAudioComponent false))
    (:NewEnumerator2
      (Development|PrintString "State:Fall")
      (AddComponent|AddAudioComponent false))
    (:NewEnumerator5
      (Development|PrintString "State:Landed")
      (AddComponent|AddAudioComponent false))))

(event EventBeginPlay
  (bind _asbp_third_person_character (Utilities|Casting|CastToBP_ThirdPersonCharacter (Game|GetPlayerCharacter 0)))
  (EventDispatchers|BindEventtoOnlocomotionStateChange _asbp_third_person_character (delegate Custom|HandleLocomotionstatechange)))

(event Collision|EventActorBeginOverlap
  (params (OtherActor :type Actor%20Object%20Reference)))

(event EventTick
  (params (DeltaSeconds :type Float%20%28single-precision%29)))

(fn ConstructionScript)